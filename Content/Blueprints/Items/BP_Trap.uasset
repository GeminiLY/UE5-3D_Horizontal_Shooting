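; BP_Trap is a looping vertical trap that damages the BP_Elysia_横版 character on contact.
; From BeginPlay, StartRun slowly raises the Cube with eased MoveComponentTo, pauses, drops it quickly, waits LoopTIme, then calls itself again.
; Rise and Fall helpers compute targets by offsetting the Cube's current relative Z up or down.
; Box begin-overlap casts the other actor to that character and applies BaseDamage.
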(event OnComponentBeginOverlap(Box)
  (params (OverlappedComponent :type Primitive%20Component%20Object%20Reference) (OtherActor :type Actor%20Object%20Reference) (OtherComp :type Primitive%20Component%20Object%20Reference) (OtherBodyIndex :type Integer) (bFromSweep :type Boolean) (SweepResult :type Hit%20Result%20Structure%20%28by%20ref%29))
  (bind _asbp_elysia_横版 (Utilities|Casting|CastToBP_Elysia_横版 OtherActor))
  (Game|Damage|ApplyDamage _asbp_elysia_横版 (Variables|Default|GetBase%20Damage) 0 0))

(event Custom|Start%20Run
  (bind _cube (Variables|Default|GetCube))
  (bind _cube_2 (Variables|Default|GetCube))
  (bind _location (CallFunction|Rise _cube_2))
  (Components|MoveComponentTo _cube_2 _location "0, 0, 0" true true 3.0 false)
  (Utilities|FlowControl|Delay 2.0)
  (bind _location_2 (CallFunction|Fall _cube))
  (Components|MoveComponentTo _cube _location_2 "0, 0, 0" false false 0.5 false)
  (Utilities|FlowControl|Delay (Variables|Default|GetLoop%20TIme))
  (CallFunction|StartRun))

(event EventBeginPlay
  (CallFunction|StartRun))

(fn ConstructionScript)

(fn Rise
  (params (Rise%20Target :type Scene%20Component%20Object%20Reference))
  (bind _relativelocation (Variables|/Script/Engine.SceneComponent|GetRelativeLocation Rise%20Target))
  (return (Math|Vector|MakeVector (.x _relativelocation) (.y _relativelocation) (+ (.z _relativelocation) 5e+02))))

(fn Fall
  (params (Fall%20Target :type Scene%20Component%20Object%20Reference))
  (bind _relativelocation (Variables|/Script/Engine.SceneComponent|GetRelativeLocation Fall%20Target))
  (return (Math|Vector|MakeVector (.x _relativelocation) (.y _relativelocation) (+ (.z _relativelocation) -5e+02))))