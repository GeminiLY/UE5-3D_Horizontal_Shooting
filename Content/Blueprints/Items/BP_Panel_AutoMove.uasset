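; Movable panel that slides between its origin and an end position, triggered by overlap or player interaction.
; A FlipFlop alternates the target of an eased MoveComponentTo over a set duration.
; Any overlap on RemoceCol starts the move through a DoOnce, which resets afterwards.
; PanelContrCol registers the panel as BP_Elysia_横版's interactive actor and toggles a hint, while MovePanel exposes the same move.
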(event OnComponentBeginOverlap(RemoceCol)
  (params (OverlappedComponent :type Primitive%20Component%20Object%20Reference) (OtherActor :type Actor%20Object%20Reference) (OtherComp :type Primitive%20Component%20Object%20Reference) (OtherBodyIndex :type Integer) (bFromSweep :type Boolean) (SweepResult :type Hit%20Result%20Structure%20%28by%20ref%29))
  (Utilities|FlowControl|DoOnce false
    (:Completed
      (CallFunction|MovetoTarget))))

(event OnComponentBeginOverlap(PanelContrCol)
  (params (OverlappedComponent :type Primitive%20Component%20Object%20Reference) (OtherActor :type Actor%20Object%20Reference) (OtherComp :type Primitive%20Component%20Object%20Reference) (OtherBodyIndex :type Integer) (bFromSweep :type Boolean) (SweepResult :type Hit%20Result%20Structure%20%28by%20ref%29))
  (bind _asbp_elysia_横版 (Utilities|Casting|CastToBP_Elysia_横版 OtherActor))
  (Default|GetInteractiveActor _asbp_elysia_横版 self)
  (Rendering|SetVisibility (Variables|Default|GetHint) true false))

(event OnComponentEndOverlap(PanelContrCol)
  (params (OverlappedComponent :type Primitive%20Component%20Object%20Reference) (OtherActor :type Actor%20Object%20Reference) (OtherComp :type Primitive%20Component%20Object%20Reference) (OtherBodyIndex :type Integer))
  (bind _asbp_elysia_横版 (Utilities|Casting|CastToBP_Elysia_横版 OtherActor))
  (Default|ClearInteractiveActor _asbp_elysia_横版)
  (Rendering|SetVisibility (Variables|Default|GetHint) false false))

(event Custom|Move%20To%20Target
  (bind _isa (Utilities|FlowControl|FlipFlop)
    (:A
      _)
    (:B
      _))
  (Components|MoveComponentTo (Variables|Default|GetPanel) (Math|Vector|SelectVector (Variables|Default|GetPosition%20End) "0, 0, 0" _isa) "0, 0, 0" true true (Variables|Default|GetMove%20Duration) false)
  (CallFunction|ResetInteraction))

(event Custom|Reset%20Interaction
  (Utilities|FlowControl|DoOnce false) ; enters at Reset
)

(event EventBeginPlay
  (Rendering|SetVisibility (Variables|Default|GetHint) false false))

(fn ConstructionScript)

(fn MovePanel
  (CallFunction|MovetoTarget))

(fn GetTeam
  (return "NewEnumerator0"))