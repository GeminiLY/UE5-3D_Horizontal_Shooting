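; BP_AIEnemy is an AI enemy pawn with health, a widget life bar, a team getter and a walk speed setter.
; Damage is reported to AI sense, then updates the bar or triggers death: ragdoll, blackboard isDead flag, OnEnemyDied call and delayed destroy.
; SearchAround loops moves to random reachable points with Y fixed at zero, but nothing here starts it.
; The OnSeePawn handler is empty.
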(event OnSeePawn(PawnSensing)
  (params (Pawn :type Pawn%20Object%20Reference)))

(event Custom|Search%20Around
  (bind _returnvalue (Transformation|GetActorLocation))
  (bind _randomlocation (AI|Navigation|GetRandomReachablePointinRadius _returnvalue 1e+03 0 0))
  ;[0.15 0.15 0.15 0.5] 搜索四周
  (AI|AIMoveTo self (Math|Vector|MakeVector (.x _randomlocation) 0.0 (.z _randomlocation)) 0 5e+01 false
    (:OnSuccess
      (Utilities|FlowControl|Delay 1.0)
      (CallFunction|SearchAround))))

(event EventBeginPlay
  (bind _asui_enemy_life_bar (Utilities|Casting|CastToUI_EnemyLifeBar (UserInterface|GetUserWidgetObject (Variables|Default|GetLife%20Bar))))
  (bind _output_get (Variables|Default|SetLife%20Bar%20Widget _asui_enemy_life_bar)))

(event Game|Damage|EventAnyDamage
  (params (Damage :type Float%20%28single-precision%29) (DamageType :type Damage%20Type%20Object%20Reference) (InstigatedBy :type Controller%20Object%20Reference) (DamageCauser :type Actor%20Object%20Reference))
  (Class|AISenseDamage|ReportDamageEvent self DamageCauser Damage (Transformation|GetActorLocation DamageCauser) "0, 0, 0" "None")
  (Variables|Default|SetHealth%20Current (- (Variables|Default|GetHealth%20Current) Damage))
  (if (<= (Variables|Default|GetHealth%20Current) 0.0)
    (Variables|Default|SetisDead true)
    (Development|SetHiddeninGame (Variables|Default|GetLife%20Bar) true false)
    (Collision|SetCollisionEnabled (Variables|Collision|GetCapsuleComponent) "NoCollision")
    (Pawn|Components|CharacterMovement|SetMovementMode (Variables|Character|GetCharacterMovement) "MOVE_None" 0)
    (Physics|SetSimulatePhysics (Variables|Character|GetMesh) true)
    (AI|Components|Blackboard|SetValueasBool (AI|GetBlackboard (AI|GetAIController self)) (Utilities|Name|MakeLiteralName "isDead") (Variables|Default|GetisDead))
    (Default|CallOnEnemyDied)
    (Utilities|FlowControl|Delay 3.0)
    (Actor|DestroyActor)
    (else
      (Default|SetLifePercentage (Variables|Default|GetLife%20Bar%20Widget) (/ (Variables|Default|GetHealth%20Current) (Variables|Default|GetHealth))))))

(fn ConstructionScript
  (Variables|Default|SetHealth%20Current (Variables|Default|GetHealth)))

(fn UpdateWalkSpeed
  (params (NewSpeed :type Float%20%28double-precision%29))
  (Variables|/Script/Engine.CharacterMovementComponent|SetMaxWalkSpeed (Variables|Character|GetCharacterMovement) NewSpeed))

(fn GetTeam
  (return (Variables|Default|GetTeam)))