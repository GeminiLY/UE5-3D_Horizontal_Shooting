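; Behavior tree task that picks a random patrol destination for a BP_AIEnemy pawn.
; It sets the enemy's walk speed to PatrolSpeed, then queries a random reachable point within PatrolRadius of the pawn.
; The point goes to the PatrolLocation blackboard key with Y forced to zero, or the pawn's current location if none is found.
; The task succeeds in either case and fails only when the pawn is not a BP_AIEnemy.
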(event EventReceiveExecuteAI
  (params (OwnerController :type AI%20Controller%20Object%20Reference) (ControlledPawn :type Pawn%20Object%20Reference))
  (bind _returnvalue (Transformation|GetActorLocation ControlledPawn))
  (bind _patrol_location (Variables|Default|GetPatrol%20Location))
  (bind _patrol_radius (Variables|Default|GetPatrol%20Radius))
  (bind (_randomlocation _returnvalue_2) (AI|Navigation|GetRandomReachablePointinRadius _returnvalue _patrol_radius 0 0))
  (bind _asbp_aienemy (Utilities|Casting|CastToBP_AIEnemy ControlledPawn)
    (:then
      (Default|UpdateWalkSpeed _asbp_aienemy (Variables|Default|GetPatrol%20Speed))
      (if _returnvalue_2
        (AI|BehaviorTree|SetBlackboardValueasVector _patrol_location (Math|Vector|MakeVector (.x _randomlocation) 0.0 (.z _randomlocation)))
        (else
          (AI|BehaviorTree|SetBlackboardValueasVector _patrol_location _returnvalue)))
      (AI|BehaviorTree|FinishExecute true))
    (:CastFailed
      (AI|BehaviorTree|FinishExecute false))))